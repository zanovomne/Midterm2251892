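; BP_Key is an interactable key pickup that records its key number on the game mode.
; BeginPlay caches a cast to Gamemode1.
; On Interact, it overwrites the game mode's Keys value with its KeyNumber, prints an acquisition message using that index into Name, then destroys itself.
; The construction script applies the Material variable to the sphere mesh, so each key's look can differ.
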(event `self.ReceiveBeginPlay`
  (bind _asgamemode_1 (cast `/Game/MidtermBase/Gamemode1` (`GameplayStatics.GetGameMode`)))
  (set `self.As Gamemode 1` _asgamemode_1))

(event `/Game/MidtermBase/BPI_Interractable.Interact`
  (bind _output_get (set `/Game/MidtermBase/Gamemode1.Keys` (`self.KeyNumber`) (`self.As Gamemode 1`)))
  (`KismetSystemLibrary.PrintString` (`KismetStringLibrary.Concat_StrStr` "Key" (`|GetArrayItem` (`self.Name`) _output_get) "Acquired"))
  (`self.K2_DestroyActor`))

(fn `UserConstructionScript`
  (`PrimitiveComponent.SetMaterial` (`self.Spehere`) 0 (`self.Material`)))